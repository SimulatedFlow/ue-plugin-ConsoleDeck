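; Demo HUD for the ConsoleDeck sample that shows players how to open the deck and reports the sample's current status on screen.
; On BeginPlay it caches the first ConsoleDeckSampleCheats actor found in the level.
; DrawHUD draws the F8 or gamepad View-button hint each frame, plus that actor's GetSampleStatus text when the reference is valid.
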(event `self.ReceiveBeginPlay`
  (bind _outactors (`GameplayStatics.GetAllActorsOfClass` "/Script/ConsoleDeck.ConsoleDeckSampleCheats"))
  (bind _asconsoledeck_sample_cheats (cast `ConsoleDeckSampleCheats` (`|GetArrayItem` _outactors)))
  (set `self.Cheats` _asconsoledeck_sample_cheats))

(event `self.ReceiveDrawHUD`
  (params (SizeX :type Integer) (SizeY :type Integer))
  (bind _cheats (`self.Cheats`))
  (`self.DrawText` "ConsoleDeck sample - press F8, or the View button on a pad, to open the deck" (make `LinearColor` 1.0 0.82 0.35 1.0) 48.0 900.0 "/Engine/EngineFonts/Roboto.Roboto" 1.3)
  (`/Engine/EditorBlueprintResources/StandardMacros.IsValid` _cheats
    (:`Is Valid`
      (`self.DrawText` (`ConsoleDeckSampleCheats.GetSampleStatus` _cheats) (make `LinearColor` 1.0 1.0 1.0 1.0) 48.0 940.0 "/Engine/EngineFonts/Roboto.Roboto" 1.2))))

(fn `UserConstructionScript`)